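; Player controller that turns Enhanced Input into camera-relative movement and look control for BP_PlayerCharacter.
; On BeginPlay it adds the movement, jump, ability and look mapping contexts and caches the character, though only movement and look are handled here.
; Look input yaws the camera arm anchor and pitches the spring arm separately.
; Movement follows the anchor's axes and snaps the mesh to its rotation with a -90 yaw offset.
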(event Input|EnhancedActionEvents|EnhancedInputActionIA_HorizontalMovements
  (params (ActionValue :type Vector%202D%20Structure) (ElapsedSeconds :type Float%20%28double-precision%29) (TriggeredSeconds :type Float%20%28double-precision%29) (InputAction :type Input%20Action%20Object%20Reference :default "/Game/MAIN/BPs/Player/Character/Inputs/InputActions/IA_HorizontalMovements.IA_HorizontalMovements"))
  (bind (_x _y) (Math|Vector2D|BreakVector2D ActionValue))
  (bind _returnvalue (Game|GetPlayerCharacter 0))
  (bind _player_character (Variables|Default|GetPlayer%20Character))
  (bind _cameraarmanchor (Variables|/Game/MAIN/BPs/Player/Character/BP_PlayerCharacter.BP_PlayerCharacter_C|GetCameraArmAnchor _player_character))
  (bind _returnvalue_2 (Transformation|GetWorldRotation _cameraarmanchor))
  (bind (_roll _pitch _yaw) (Math|Rotator|BreakRotator _returnvalue_2))
  (Pawn|Input|AddMovementInput _returnvalue (* _y (Math|Vector|GetRightVector (Transformation|GetWorldRotation (Variables|/Game/MAIN/BPs/Player/Character/BP_PlayerCharacter.BP_PlayerCharacter_C|GetCameraArmAnchor (Variables|Default|GetPlayer%20Character))))) 1.0 false)
  (Pawn|Input|AddMovementInput _returnvalue (* _x (Math|Vector|GetForwardVector _returnvalue_2)) 1.0 false)
  (Transformation|SetWorldRotation (Variables|/Script/Engine.Character|GetMesh (Variables|Default|GetPlayer%20Character)) (Math|Rotator|MakeRotator _roll _pitch (+ _yaw -9e+01)) false false))

(event Input|EnhancedActionEvents|EnhancedInputActionIA_MechaLook
  (params (ActionValue :type Vector%202D%20Structure) (ElapsedSeconds :type Float%20%28double-precision%29) (TriggeredSeconds :type Float%20%28double-precision%29) (InputAction :type Input%20Action%20Object%20Reference :default "/Game/MAIN/BPs/Player/Character/Inputs/InputActions/IA_MechaLook.IA_MechaLook"))
  (bind (_x _y) (Math|Vector2D|BreakVector2D ActionValue))
  (bind _player_character (Variables|Default|GetPlayer%20Character))
  (Transformation|AddLocalRotation (Variables|/Game/MAIN/BPs/Player/Character/BP_PlayerCharacter.BP_PlayerCharacter_C|GetCameraArmAnchor _player_character) (Math|Rotator|MakeRotator 0.0 0.0 _x) false false)
  (Transformation|AddLocalRotation (Variables|/Game/MAIN/BPs/Player/Character/BP_PlayerCharacter.BP_PlayerCharacter_C|GetSpringArm _player_character) (Math|Rotator|MakeRotator 0.0 _y 0.0) false false))

(event EventBeginPlay
  (bind _returnvalue (PlayerController|LocalPlayerSubsystems|GetEnhancedInputLocalPlayerSubsystem))
  (Input|AddMappingContext _returnvalue "/Game/MAIN/BPs/Player/Character/Inputs/IMC_BasicHorizontalMovements.IMC_BasicHorizontalMovements" 0 "(bIgnoreAllPressedKeysUntilRelease=True,bForceImmediately=False,bNotifyUserSettings=False)")
  (Input|AddMappingContext _returnvalue "/Game/MAIN/BPs/Player/Character/Inputs/IMC_Jump.IMC_Jump" 0 "(bIgnoreAllPressedKeysUntilRelease=True,bForceImmediately=False,bNotifyUserSettings=False)")
  (Input|AddMappingContext _returnvalue "/Game/MAIN/BPs/Player/Character/Inputs/IMC_AbilityInputs.IMC_AbilityInputs" 0 "(bIgnoreAllPressedKeysUntilRelease=True,bForceImmediately=False,bNotifyUserSettings=False)")
  (Input|AddMappingContext _returnvalue "/Game/MAIN/BPs/Player/Character/Inputs/IMC_MechaLook.IMC_MechaLook" 0 "(bIgnoreAllPressedKeysUntilRelease=True,bForceImmediately=False,bNotifyUserSettings=False)")
  (bind _asbp_player_character (Utilities|Casting|CastToBP_PlayerCharacter (Game|GetPlayerCharacter 0)))
  (Variables|Default|SetPlayer%20Character _asbp_player_character))

(fn ConstructionScript)